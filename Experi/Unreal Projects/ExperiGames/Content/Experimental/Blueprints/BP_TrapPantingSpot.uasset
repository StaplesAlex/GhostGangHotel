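; BP_TrapPantingSpot is an experimental world spot that marks where the player can plant a trap.
; BeginPlay gives its Boxes component a random yaw and caches a BP_PlayerManOLD reference that is not otherwise used here, while Tick turns the prompt Widget toward the player pawn.
; Box overlaps with BP_NewPlayerMan show or hide the Widget and toggle Plantable on the player's BP_PlayerCameraThing pawn.
; TrapPlanted is an empty event.
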(event OnComponentBeginOverlap(Box)
  (params (OverlappedComponent :type Primitive%20Component%20Object%20Reference) (OtherActor :type Actor%20Object%20Reference) (OtherComp :type Primitive%20Component%20Object%20Reference) (OtherBodyIndex :type Integer) (bFromSweep :type Boolean) (SweepResult :type Hit%20Result%20Structure%20%28by%20ref%29))
  (if (== (Utilities|GetClass OtherActor) "/Game/Experimental/Blueprints/BP_NewPlayerMan.BP_NewPlayerMan_C")
    (Rendering|SetVisibility (Variables|Default|GetWidget) true false)
    (bind _asbp_player_camera_thing (Utilities|Casting|CastToBP_PlayerCameraThing (Game|Player|GetPlayerPawn 0)))
    (Variables|/Game/Experimental/Blueprints/BP_PlayerCameraThing.BP_PlayerCameraThing_C|SetPlantable _asbp_player_camera_thing true)))

(event OnComponentEndOverlap(Box)
  (params (OverlappedComponent :type Primitive%20Component%20Object%20Reference) (OtherActor :type Actor%20Object%20Reference) (OtherComp :type Primitive%20Component%20Object%20Reference) (OtherBodyIndex :type Integer))
  (if (== (Utilities|GetClass OtherActor) "/Game/Experimental/Blueprints/BP_NewPlayerMan.BP_NewPlayerMan_C")
    (Rendering|SetVisibility (Variables|Default|GetWidget) false false)
    (bind _asbp_player_camera_thing (Utilities|Casting|CastToBP_PlayerCameraThing (Game|Player|GetPlayerPawn 0)))
    (Variables|/Game/Experimental/Blueprints/BP_PlayerCameraThing.BP_PlayerCameraThing_C|SetPlantable _asbp_player_camera_thing false)))

(event Custom|TrapPlanted)

(event EventBeginPlay
  (bind _outactors (Actor|GetAllActorsOfClass "/Game/Experimental/Blueprints/BP_PlayerManOLD.BP_PlayerManOLD_C"))
  (Variables|Default|SetPlayerMan (Utilities|Array|Get(acopy) _outactors))
  (Transformation|SetRelativeRotation (Variables|Default|GetBoxes) (Math|Rotator|MakeRotator 0.0 0.0 (Math|Random|RandomFloatinRange 0.0 3.6e+02)) false false))

(event EventTick
  (params (DeltaSeconds :type Float%20%28single-precision%29))
  (Transformation|SetWorldRotation (Variables|Default|GetWidget) (Math|Rotator|FindLookatRotation (Transformation|GetActorLocation) (Transformation|GetActorLocation (Game|Player|GetPlayerPawn 0))) false false))

(fn ConstructionScript)