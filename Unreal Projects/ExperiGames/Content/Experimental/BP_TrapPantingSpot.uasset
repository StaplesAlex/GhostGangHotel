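; BP_TrapPantingSpot is an experimental trap-spot actor that shows an indicator when the player is nearby.
; BeginPlay caches the first BP_PlayerMan and the first BP_TrapSpot widget found globally, rather than the actor's own widget instance.
; Each Tick turns its Widget component toward the player pawn and toggles the cached widget's desired opacity by a distance check to BP_PlayerMan.
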(event EventBeginPlay
  (bind _outactors (Actor|GetAllActorsOfClass "/Game/Experimental/BP_PlayerMan.BP_PlayerMan_C"))
  (Variables|Default|SetPlayerMan (Utilities|Array|Get(acopy) _outactors))
  (bind _foundwidgets (Widget|GetAllWidgetsOfClass "/Game/Experimental/BP_TrapSpot.BP_TrapSpot_C" false))
  (Variables|Default|SetIndicatorWidget (Utilities|Array|Get(acopy) _foundwidgets)))

(event Collision|EventActorBeginOverlap
  (params (OtherActor :type Actor%20Object%20Reference)))

(event EventTick
  (params (DeltaSeconds :type Float%20%28single-precision%29))
  (bind _returnvalue (Transformation|GetActorLocation))
  (bind _indicatorwidget (Variables|Default|GetIndicatorWidget))
  (Transformation|SetWorldRotation (Variables|Default|GetWidget) (Math|Rotator|FindLookatRotation _returnvalue (Transformation|GetActorLocation (Game|Player|GetPlayerPawn 0))) false false)
  (if (<= (Math|Vector|Distance(Vector) _returnvalue (Transformation|GetActorLocation (Variables|Default|GetPlayerMan))) 5e+02)
    (Variables|/Game/Experimental/BP_TrapSpot.BP_TrapSpot_C|SetDesiredOpacity _indicatorwidget 1.0)
    (else
      (Variables|/Game/Experimental/BP_TrapSpot.BP_TrapSpot_C|SetDesiredOpacity _indicatorwidget 0.0))))

(fn ConstructionScript)