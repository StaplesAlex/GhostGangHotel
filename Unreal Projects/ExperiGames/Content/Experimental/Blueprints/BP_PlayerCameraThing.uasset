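; Experimental player camera that pans along its right and up vectors on input axes and gives click-to-move orders to the first BP_NewPlayerMan in the level.
; It shows the mouse cursor; left click spawns a move marker at the cursor's trace hit and starts the character moving there, while right click resets its position.
; When Plantable, Tick times a held use key via the E key and spawns a small explosion at the cursor around three seconds.
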(event EventBeginPlay
  (Variables|/Script/Engine.PlayerController|SetbShowMouseCursor (Game|GetPlayerController 0) true)
  (bind _outactors (Actor|GetAllActorsOfClass "/Game/Experimental/Blueprints/BP_NewPlayerMan.BP_NewPlayerMan_C"))
  (Variables|Default|SetPlayerCharacter (Utilities|Array|Get(acopy) _outactors)))

(event Collision|EventActorBeginOverlap
  (params (OtherActor :type Actor%20Object%20Reference)))

(event EventTick
  (params (DeltaSeconds :type Float%20%28single-precision%29))
  (if (Variables|Default|GetPlantable)
    (if (Variables|Default|GetMouseDown)
      (bind _output_get (Variables|Default|SetHoldTime (Class|PlayerController|GetInputKeyTimeDown (Game|GetPlayerController 0) "E")))
      (if (Math|Float|NearlyEqual(Float) _output_get 3.0 0.1)
        (Effects|SpawnEmitteratLocation "/Game/StarterContent/Particles/P_Explosion.P_Explosion" (.Location (Collision|BreakHitResult (.HitResult (Game|Player|GetHitResultUnderCursorbyChannel (Game|GetPlayerController 0) "TraceTypeQuery1" true)))) "0, 0, 0" "0.100000,0.100000,0.100000"))
      (else
        (Variables|Default|SetHoldTime 0.0)))))

(event Input|ActionEvents|InputActionUseKey
  (params (Key :type Key%20Structure :default "None"))
  (:Pressed
    (Variables|Default|SetMouseDown true))
  (:Released
    (Variables|Default|SetMouseDown false)))

(event Input|AxisEvents|InputAxisLeft/Right
  (params (AxisValue :type Float%20%28single-precision%29))
  (Transformation|AddActorWorldOffset (* (Transformation|GetActorRightVector) (* AxisValue (Variables|Default|GetCamMoveSpeed)))))

(event Input|AxisEvents|InputAxisUp/Down
  (params (AxisValue :type Float%20%28single-precision%29))
  (Transformation|AddActorWorldOffset (* (Transformation|GetActorUpVector) (* AxisValue (Variables|Default|GetCamMoveSpeed)))))

(event Input|MouseEvents|LeftMouseButton
  (params (Key :type Key%20Structure :default "None"))
  (bind _returnvalue (Game|GetPlayerController 0))
  (bind _hitresult (Game|Player|GetHitResultUnderCursorbyChannel _returnvalue "TraceTypeQuery1" true))
  (bind _location (Collision|BreakHitResult _hitresult))
  (:Pressed
    (Niagara|SpawnSystematLocation "/Game/Experimental/GuyMoveHereFX.GuyMoveHereFX" _location)
    (Default|StartMoving (Variables|Default|GetPlayerCharacter) _location)))

(event Input|MouseEvents|RightMouseButton
  (params (Key :type Key%20Structure :default "None"))
  (:Pressed
    (Default|ResetPos (Variables|Default|GetPlayerCharacter))))

(fn ConstructionScript)