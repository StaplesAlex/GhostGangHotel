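; BP_NewPlayerMan is a controllable character that moves to commanded locations and can show a world-space loading bar.
; StartMoving, blocked while Planting, uses SimpleMoveToLocation and spawns a destination effect snapped to one of two heights.
; EnableBar and DisableBar create and destroy a LoadingBar widget component at runtime.
; While that widget exists, Tick rotates it toward the player character and halts character movement if Planting.
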(event Custom|ResetPos
  (Components|Movement|StopMovementImmediately (Variables|Default|GetFloatingPawnMovement))
  (Transformation|SetActorLocation "0, 0,200.000000" false true))

(event Custom|Start%20Moving
  (params (Location :type Vector))
  (bind (_x _y _z) (Math|Vector|BreakVector Location))
  (if (not (Variables|Default|GetPlanting))
    (AI|Navigation|SimpleMovetoLocation (Pawn|GetController) Location)
    (if (> _z 4e+02)
      (Niagara|SpawnSystematLocation "/Game/GhostGang/Particle_Effects/DesiredLocationEffect.DesiredLocationEffect" (Math|Vector|MakeVector _x _y 4.5e+02))
      (else
        (Niagara|SpawnSystematLocation "/Game/GhostGang/Particle_Effects/DesiredLocationEffect.DesiredLocationEffect" (Math|Vector|MakeVector _x _y 0.0))))))

(event Custom|Enable%20Bar
  (bind _returnvalue (AddComponent|AddWidgetComponent false (Math|Transform|MakeTransform "0, 0,190.000000" "0, 0, 0" "1,6.000000,3.000000")))
  (bind _output_get (Variables|Default|SetWidgy _returnvalue))
  (Class|WidgetComponent|SetDrawatDesiredSize _output_get true)
  (bind _returnvalue_2 (UserInterface|CreateWidget "/Game/GhostGang/BP/WDGT/InGame/LoadingBar.LoadingBar_C"))
  (UserInterface|SetWidget _output_get _returnvalue_2))

(event Custom|Disable%20Bar
  (Components|DestroyComponent (Variables|Default|GetWidgy)))

(event Custom|Stop%20Moving
  (Components|Movement|StopMovementImmediately (Variables|Default|GetFloatingPawnMovement)))

(event EventBeginPlay)

(event Collision|EventActorBeginOverlap
  (params (OtherActor :type Actor%20Object%20Reference)))

(event EventTick
  (params (DeltaSeconds :type Float%20%28single-precision%29))
  (bind _widgy (Variables|Default|GetWidgy))
  (Utilities|IsValid _widgy
    (:Is%20Valid
      (Transformation|SetWorldRotation _widgy (Math|Rotator|FindLookatRotation (Transformation|GetWorldLocation _widgy) (Transformation|GetActorLocation (Game|GetPlayerCharacter 0))) false false)
      (if (Variables|Default|GetPlanting)
        (Components|Movement|StopMovementImmediately (Variables|Character|GetCharacterMovement))))))

(fn ConstructionScript)