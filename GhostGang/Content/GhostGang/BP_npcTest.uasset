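; BP_npcTest is a test NPC in GhostGang that wanders the navmesh and detects being caught.
; A looping four-second timer sends it via SimpleMoveToLocation to a random navigable point around the world origin, unless Lost is set.
; A Box overlap with a matching actor class only prints a red "CAUGHT" message.
; The node that sets Lost is disconnected, so nothing here stops the wandering.
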(event OnComponentBeginOverlap(Box)
  (params (OverlappedComponent :type Primitive%20Component%20Object%20Reference) (OtherActor :type Actor%20Object%20Reference) (OtherComp :type Primitive%20Component%20Object%20Reference) (OtherBodyIndex :type Integer) (bFromSweep :type Boolean) (SweepResult :type Hit%20Result%20Structure%20%28by%20ref%29))
  (if (== (Utilities|GetClass OtherActor) 0)
    (Development|PrintText "CAUGHT" true true "(R=1.000000,G=0.000000,B=0.000000,A=1.000000)")))

(event Custom|move
  (if (not (Variables|Default|GetLost?))
    (bind _randomlocation (Class|NavigationSystemV1|GetRandomLocationinNavigableRadius (Math|Vector|VectorZero) 7e+02 0 0))
    (AI|Navigation|SimpleMovetoLocation (Pawn|GetController) _randomlocation)))

(event EventBeginPlay
  (Utilities|Time|SetTimerbyEvent (delegate Custom|move) 4.0 true))

(event Collision|EventActorBeginOverlap
  (params (OtherActor :type Actor%20Object%20Reference)))

(event EventTick
  (params (DeltaSeconds :type Float%20%28single-precision%29)))

(fn ConstructionScript)